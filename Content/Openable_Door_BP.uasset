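; Openable door Actor that swings open and shut in response to the OnOpen and OnClose events from OpenDoor.
; The Door_Swing timeline plays forward to open and in reverse to close, adding its OpenAngle yaw to the rotation cached at BeginPlay.
; A Sound Timing event track on the same timeline plays the door lock sound at the cached actor location.
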(event OnClose(OpenDoor)
  (bind _openangle (Timeline|Door_Swing Reverse)
    (:Update
      _)
    (:Sound%20Timing
      (Audio|PlaySoundatLocation "/Game/Audio/door-lock.door-lock" (Variables|Default|GetActorLocation) "0, 0, 0" 0.5)))
  (Transformation|SetActorRotation (Math|Rotator|CombineRotators (Math|Rotator|MakeRotator 0.0 0.0 _openangle) (Variables|Default|GetInitialRotation))))

(event OnOpen(OpenDoor)
  (bind _openangle (Timeline|Door_Swing Play)
    (:Update
      _)
    (:Sound%20Timing
      (Audio|PlaySoundatLocation "/Game/Audio/door-lock.door-lock" (Variables|Default|GetActorLocation) "0, 0, 0" 0.5)))
  (Transformation|SetActorRotation (Math|Rotator|CombineRotators (Math|Rotator|MakeRotator 0.0 0.0 _openangle) (Variables|Default|GetInitialRotation))))

(event EventBeginPlay
  (Variables|Default|SetInitialRotation (Transformation|GetActorRotation))
  (Variables|Default|SetActorLocation (Transformation|GetActorLocation)))

(fn ConstructionScript)